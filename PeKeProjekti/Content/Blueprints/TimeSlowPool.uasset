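; TimeSlowPool manages a capped pool of TimeSlow actors that fall down the screen along the world Z axis.
; CreateTimeSlow spawns one at a random X at the start height and adds it to the pool until the maximum is reached.
; UpdateTimeSlows lowers each by its Speed per call, recycling those below the negated start height to the top with a new X and reset speed.
; Its event graph is empty, so both functions rely on external callers.
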(fn `CreateTimeSlow`
  (if (< (`self.numberOfTimeSlows`) (`self.maxNumberofTimeSlows`))
    (bind _returnvalue (`|SpawnActorFromClass` "/Game/Blueprints/TimeSlow.TimeSlow_C" (`KismetMathLibrary.MakeTransform` (`KismetMathLibrary.MakeVector` (`KismetMathLibrary.RandomFloatInRange` -900.0 1800.0) 0.0 (`self.timeSlowStartZ`))) "Undefined" "OverrideRootScale" null null))
    (set `/Game/Blueprints/TimeSlow.Speed` (`/Game/Blueprints/TimeSlow.Speed` _returnvalue) _returnvalue)
    (`KismetArrayLibrary.Array_Insert` (`self.timeSlowPool`) _returnvalue (`self.numberOfTimeSlows`))
    (`/Engine/EditorBlueprintResources/StandardMacros.IncrementInt` (`self.numberOfTimeSlows`))))

(fn `UpdateTimeSlows`
  (locals (arrayElement :type "PaperSpriteActor Object Reference") (arrayIndex :type Integer))
  (for (_array_element _array_index) (`self.timeSlowPool`)
    (set `local.arrayElement` _array_element)
    (set `local.arrayIndex` _array_index)
    (bind _rootcomponent (`Actor.RootComponent` _array_element))
    (if (< (.z (`SceneComponent.K2_GetComponentLocation` _rootcomponent)) (- 0.0 (`self.timeSlowStartZ`)))
      (`SceneComponent.K2_SetWorldLocation` (`Actor.RootComponent` (`local.arrayElement`)) (`KismetMathLibrary.MakeVector` (`KismetMathLibrary.RandomFloatInRange` -900.0 1800.0) 0.0 (`self.timeSlowStartZ`)) false false)
      (bind _astime_slow (cast `/Game/Blueprints/TimeSlow` (`local.arrayElement`)))
      (set `/Game/Blueprints/TimeSlow.Speed` 20.0 _astime_slow)
      (else
        (bind _astime_slow_2 (cast `/Game/Blueprints/TimeSlow` _array_element))
        (`SceneComponent.K2_AddWorldOffset` _rootcomponent (`KismetMathLibrary.MakeVector` 0.0 0.0 (- 0.0 (`/Game/Blueprints/TimeSlow.Speed` _astime_slow_2))) false false)))))

(fn `UserConstructionScript`)