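; EnergyheartPool manages a capped pool of Energyheart actors that scroll along negative X and are recycled rather than destroyed.
; CreateEnergyheart spawns a heart at the start X with random height and a time-dependent random speed, then stores it in HeartPool.
; UpdateEnergyhearts moves each heart by its Speed per call, wrapping those past the opposite X bound with new height and speed.
; Its event graph is empty, so both functions rely on external callers.
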(fn `CreateEnergyheart`
  (if (< (`self.numberOfEnergyhearts`) (`self.maxNumberofEnergyhearts`))
    (bind _returnvalue (`|SpawnActorFromClass` "/Game/Blueprints/Energyheart.Energyheart_C" (`KismetMathLibrary.MakeTransform` (`KismetMathLibrary.MakeVector` (`self.energyheartStartX`) 0.0 (`KismetMathLibrary.RandomFloatInRange` 0.0 300.0))) "Undefined" "OverrideRootScale" null null))
    (bind _speed (`/Game/Blueprints/Energyheart.Speed` _returnvalue))
    (set `/Game/Blueprints/Energyheart.Speed` (`KismetMathLibrary.RandomFloatInRange` (/ _speed (/ (`KismetSystemLibrary.GetGameTimeInSeconds`) 2.0)) _speed) _returnvalue)
    (`KismetArrayLibrary.Array_Insert` (`self.heartPool`) _returnvalue (`self.numberOfEnergyhearts`))
    (`/Engine/EditorBlueprintResources/StandardMacros.IncrementInt` (`self.numberOfEnergyhearts`))))

(fn `UpdateEnergyhearts`
  (locals (arrayElement :type "PaperSpriteActor Object Reference") (arrayIndex :type Integer))
  (for (_array_element _array_index) (`self.heartPool`)
    (set `local.arrayElement` _array_element)
    (set `local.arrayIndex` _array_index)
    (bind _rootcomponent (`Actor.RootComponent` _array_element))
    (if (< (.x (`SceneComponent.K2_GetComponentLocation` _rootcomponent)) (- 0.0 (`self.energyheartStartX`)))
      (`SceneComponent.K2_SetWorldLocation` (`Actor.RootComponent` (`local.arrayElement`)) (`KismetMathLibrary.MakeVector` (`self.energyheartStartX`) 0.0 (`KismetMathLibrary.RandomFloatInRange` -200.0 100.0)) false false)
      (bind _asenergyheart (cast `/Game/Blueprints/Energyheart` (`local.arrayElement`)))
      (set `/Game/Blueprints/Energyheart.Speed` (`KismetMathLibrary.RandomFloatInRange` 20.0 35.0) _asenergyheart)
      (else
        (bind _asenergyheart_2 (cast `/Game/Blueprints/Energyheart` _array_element))
        (`SceneComponent.K2_AddWorldOffset` _rootcomponent (`KismetMathLibrary.MakeVector` (- 0.0 (`/Game/Blueprints/Energyheart.Speed` _asenergyheart_2))) false false)))))

(fn `UserConstructionScript`)