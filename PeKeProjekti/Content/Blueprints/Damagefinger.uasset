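; Damagefinger is a hazard actor that drains the player character's LifeForce when its Box component is overlapped.
; The overlap event identifies MyCharacter_1 by display name and cast, then subtracts Effect, clamping LifeForce at zero.
; If LifeForce was above zero, it also plays a hit sound at world origin, shows DamageText in the GameLevelHUD header and sets its Speed variable high.
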(event `self.Box.OnComponentBeginOverlap`
  (params (OverlappedComponent :type "PrimitiveComponent Object Reference") (OtherActor :type "Actor Object Reference") (OtherComp :type "PrimitiveComponent Object Reference") (OtherBodyIndex :type Integer) (bFromSweep :type Boolean) (SweepResult :type "HitResult Structure (by ref)"))
  ;[1 1 1] Check if collide with character
  (if (`KismetStringLibrary.EqualEqual_StrStr` (`KismetSystemLibrary.GetDisplayName` OtherActor) "MyCharacter_1")
    (bind _asmy_character_1 (cast `/Game/Blueprints/MyCharacter_1` OtherActor))
    (bind _lifeforce (`/Game/Blueprints/MyCharacter_1.lifeForce` _asmy_character_1))
    ;[1 1 1] Check whether life force is not on maximum already before boost
    (if (> _lifeforce 0.0)
      (bind _returnvalue (- _lifeforce (`self.Effect`)))
      ;[1 1 1] Check whether sum of boost and life force is on maximum
      (if (>= _returnvalue 0.0)
        (set `/Game/Blueprints/MyCharacter_1.lifeForce` _returnvalue _asmy_character_1)
        (else
          (set `/Game/Blueprints/MyCharacter_1.lifeForce` 0.0 _asmy_character_1)))
      ;[1 1 1] Play sound, set GameLevelHUD's HeaderText and increase speed a lot
      (`GameplayStatics.PlaySoundAtLocation` "/Game/Sounds/270332__littlerobotsoundfactory__hit-03.270332__littlerobotsoundfactory__hit-03" (0.0 0.0 0.0) (struct) 1.0 1.0 0.0 null null null)
      (`TextBlock.SetText` (`/Game/GUIs/GameLevelHUD.HeaderText` (`self.GameLevelHUD`)) (`KismetTextLibrary.Conv_StringToText` (`self.DamageText`)))
      (set `self.Speed` 500.0))))

(fn `UserConstructionScript`)