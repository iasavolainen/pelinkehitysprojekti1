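; DamagefingerPool manages a recycled pool of Damagefinger collectibles that scroll from right to left across the screen.
; CreateCollectible spawns one at the right edge with random height and time-dependent random speed, until the pool reaches its maximum.
; UpdateCollectibles shifts each one left by its Speed per call, wrapping those past the left limit back right with new height and speed.
; Its event graph is empty, so both functions rely on external callers.
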(fn `CreateCollectible`
  ;[1 1 1] Only create collectible if max amount has not been reached
  (if (< (`self.numberofCollectibles`) (`self.maxNumberofCollectibles`))
    ;[1 1 1] Create collectible into the scene and adjust its position and speed
    (bind _returnvalue (`|SpawnActorFromClass` "/Game/Blueprints/Damagefinger.Damagefinger_C" (`KismetMathLibrary.MakeTransform` (`KismetMathLibrary.MakeVector` (`self.collectibleStartX`) 0.0 (`KismetMathLibrary.RandomFloatInRange` -200.0 100.0))) "Undefined" "OverrideRootScale" null null))
    (bind _speed (`/Game/Blueprints/Damagefinger.Speed` _returnvalue))
    (set `/Game/Blueprints/Damagefinger.Speed` (`KismetMathLibrary.RandomFloatInRange` (/ _speed (/ (`KismetSystemLibrary.GetGameTimeInSeconds`) 2.0)) _speed) _returnvalue)
    ;[1 1 1] Add created collectible to the pool and increment counter
    (`KismetArrayLibrary.Array_Insert` (`self.thePool`) _returnvalue (`self.numberofCollectibles`))
    (`/Engine/EditorBlueprintResources/StandardMacros.IncrementInt` (`self.numberofCollectibles`))))

(fn `UpdateCollectibles`
  (locals (arrayElement :type "PaperSpriteActor Object Reference") (arrayIndex :type Integer))
  ;[1 1 1] Update each collectible in the pool
  (for (_array_element _array_index) (`self.thePool`)
    ;[1 1 1] Check whether collectible has travelled far enough to the left of the screen in order to be valid for reappearing again from the right of the screen
    (set `local.arrayElement` _array_element)
    (set `local.arrayIndex` _array_index)
    (bind _rootcomponent (`Actor.RootComponent` _array_element))
    (if (< (.x (`SceneComponent.K2_GetComponentLocation` _rootcomponent)) (- 0.0 (`self.collectibleStartX`)))
      ;[1 1 1] Create collectible into the scene and adjust its position and speed
      (`SceneComponent.K2_SetWorldLocation` (`Actor.RootComponent` (`local.arrayElement`)) (`KismetMathLibrary.MakeVector` (`self.collectibleStartX`) 0.0 (`KismetMathLibrary.RandomFloatInRange` -200.0 100.0)) false false)
      (bind _asdamagefinger (cast `/Game/Blueprints/Damagefinger` (`local.arrayElement`)))
      (set `/Game/Blueprints/Damagefinger.Speed` (`KismetMathLibrary.RandomFloatInRange` 20.0 30.0) _asdamagefinger)
      (else
        ;[1 1 1] If not too far on the left, just move the collectible
        (bind _asdamagefinger_2 (cast `/Game/Blueprints/Damagefinger` _array_element))
        (`SceneComponent.K2_AddWorldOffset` _rootcomponent (`KismetMathLibrary.MakeVector` (- 0.0 (`/Game/Blueprints/Damagefinger.Speed` _asdamagefinger_2))) false false)))))

(fn `UserConstructionScript`)