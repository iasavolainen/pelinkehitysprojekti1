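; TimeSlow is a trigger actor that applies a time-slow effect to the player character on contact.
; Sphere overlap identifies MyCharacter_1 by display name, casts it, records the effect start time on it and sets its CustomTimeDilation from the TimeSlow variable.
; It also plays a clock tick sound, shows the slow message in the HUD header and sets its own Speed variable.
; Nothing in this Blueprint reverts the effect.
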(event `self.Sphere.OnComponentBeginOverlap`
  (params (OverlappedComponent :type "PrimitiveComponent Object Reference") (OtherActor :type "Actor Object Reference") (OtherComp :type "PrimitiveComponent Object Reference") (OtherBodyIndex :type Integer) (bFromSweep :type Boolean) (SweepResult :type "HitResult Structure (by ref)"))
  (if (`KismetStringLibrary.EqualEqual_StrStr` (`KismetSystemLibrary.GetDisplayName` OtherActor) "MyCharacter_1")
    (bind _asmy_character_1 (cast `/Game/Blueprints/MyCharacter_1` OtherActor))
    (set `/Game/Blueprints/MyCharacter_1.effectStartTime` (`KismetSystemLibrary.GetGameTimeInSeconds`) _asmy_character_1)
    (set `Actor.CustomTimeDilation` (`self.timeSlow`) _asmy_character_1)
    (`GameplayStatics.PlaySoundAtLocation` "/Game/Sounds/clocktick.clocktick" (0.0 0.0 0.0) (struct) 0.7 1.0 0.0 null null null)
    (`TextBlock.SetText` (`/Game/GUIs/GameLevelHUD.HeaderText` (`self.GameLevelHUD`)) (`KismetTextLibrary.Conv_StringToText` (`self.SlowText`)))
    (set `self.Speed` 500.0)))

(fn `UserConstructionScript`)